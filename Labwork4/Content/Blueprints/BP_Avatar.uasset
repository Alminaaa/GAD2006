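; BP_Avatar is a networked player avatar with a wall-targeted dash for the Red team.
; Each Tick reads the team via NetPlayerState and, for Red, traces forward for an actor tagged "wall", drawing debug lines.
; A hit enables dashing and stores a destination pulled back by the capsule radius at current height.
; Dash input enters a DoOnce with no visible movement logic; AllowDash resets it, restoring movement scale and Tick.
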(event `self.ReceiveTick`
  (params (DeltaSeconds :type "Float (single-precision)"))
  (bind _returnvalue (`self.K2_GetActorLocation`))
  (bind (_returnvalue_x _returnvalue_y _returnvalue_z) (`KismetMathLibrary.BreakVector` (`self.K2_GetActorLocation`)))
  (set `self.DashOK` false)
  (`self.Pstate`)
  (switch `EPlayerTeam` "TEAM_Unknown"
    (:`TEAM_Red`
      (bind (_outhit _returnvalue_2) (`KismetSystemLibrary.LineTraceSingle` :`Start` _returnvalue :`End` (+ _returnvalue (* (`self.GetActorForwardVector`) 3000.0)) :`TraceChannel` "TraceTypeQuery1" :`DrawDebugType` "ForDuration" :`DrawTime` 0.1))
      (if _returnvalue_2
        (bind (_bblockinghit _binitialoverlap _time _distance _location _impactpoint _normal _impactnormal _physmat _hitactor) (`GameplayStatics.BreakHitResult` _outhit))
        (if (`self.ActorHasTag` _hitactor "wall")
          (set `self.DashDistance` _distance)
          (set `self.DashDestination` (`KismetMathLibrary.MakeVector` (.x (- _location (* (`self.GetActorForwardVector`) (`CapsuleComponent.CapsuleRadius` (`self.CapsuleComponent`))))) (.y (- _location (* (`self.GetActorForwardVector`) (`CapsuleComponent.CapsuleRadius` (`self.CapsuleComponent`))))) _returnvalue_z))
          (set `self.DashOK` true))))))

(event `InputAction|Dash`
  (params (Key :type "Key Structure"))
  (:`Pressed`
    (if (`self.DashOK`)
      (`/Engine/EditorBlueprintResources/StandardMacros.DoOnce` false :!label _label))))

(event `AllowDash`
  (set `self.MovementScale` 1.0)
  (`self.SetActorTickEnabled` true)
  (goto _label :!via `Reset`))

(fn `UserConstructionScript`)